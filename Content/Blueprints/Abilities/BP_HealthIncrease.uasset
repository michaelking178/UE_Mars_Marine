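; BP_HealthIncrease is an ability that permanently raises the player marine's maximum health by a fixed amount.
; On BeginPlay, if activated, it casts the player pawn to BP_Marine and registers itself in that marine's AbilitySet active abilities.
; It then calls ApplyEffect, which adds the bonus to MaxHealth without changing current health or providing any removal logic.
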(event EventBeginPlay
  (if (Variables|Default|GetIs%20Activated)
    (bind _asbp_marine (Utilities|Casting|CastToBP_Marine (Game|Player|GetPlayerPawn 0)))
    (bind _output_get (Variables|Default|SetMarine _asbp_marine))
    (Utilities|Array|Add (Variables|/Game/Blueprints/Abilities/C_Abilities.C_Abilities_C|GetActive%20Abilities (Variables|/Game/Blueprints/Pawns/BP_Marine.BP_Marine_C|GetAbility%20Set _output_get)) self)
    (CallFunction|ApplyEffect)))

(fn ConstructionScript
  (|CallParentFunction))

(fn ApplyEffect
  (bind _marine (Variables|Default|GetMarine))
  (Variables|/Game/Blueprints/Pawns/BP_Marine.BP_Marine_C|SetMax%20Health _marine (+ (Variables|/Game/Blueprints/Pawns/BP_Marine.BP_Marine_C|GetMax%20Health _marine) 25.0)))