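; BP_Armory is an interactable armory actor that shows an on-screen prompt while the player is near it.
; On BeginPlay it creates a W_ArmoryPrompt widget for the first player controller, adds it to the viewport and hides it.
; Actor begin and end overlap events with the player pawn toggle the prompt between visible and hidden.
; It contains no interaction logic beyond the prompt.
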(event EventBeginPlay
  (bind _returnvalue (UserInterface|CreateWidget "/Game/UI/AbilityMenus/W_ArmoryPrompt.W_ArmoryPrompt_C" (Game|GetPlayerController 0)))
  (bind _output_get (Variables|Default|SetW_ArmoryPrompt _returnvalue))
  (UserInterface|Viewport|AddtoViewport _output_get 0)
  (Widget|SetVisibility _output_get "Hidden"))

(event Collision|EventActorBeginOverlap
  (params (OtherActor :type Actor%20Object%20Reference))
  (if (== OtherActor (Game|Player|GetPlayerPawn 0))
    (Widget|SetVisibility (Variables|Default|GetW_ArmoryPrompt) "Visible")))

(event EventTick
  (params (DeltaSeconds :type Float%20%28single-precision%29)))

(event Collision|EventActorEndOverlap
  (params (OtherActor :type Actor%20Object%20Reference))
  (if (== OtherActor (Game|Player|GetPlayerPawn 0))
    (Widget|SetVisibility (Variables|Default|GetW_ArmoryPrompt) "Hidden")))

(fn ConstructionScript)