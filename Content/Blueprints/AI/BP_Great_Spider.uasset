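; Great Spider enemy AI that chases the marine and wanders to a random TargetPoint once the player dies.
; BeginPlay loops AIMoveTo, while Tick halts movement for an attack montage in range; DamagePlayer is not called within this Blueprint.
; At zero health it disables collision, awards kill and experience, may drop a health pickup, then is destroyed after a delay.
; RemoveSpiderFromArray casts the game mode, but its RegisterSpiderDeath call is unconnected.
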(event EventBeginPlay
  (if (CallFunction|IsAlive) :!label _label
    (if (CallFunction|IsPlayerAlive)
      (Utilities|MovetoPlayer)
      (goto _label)
      (else
        (Utilities|MovetoRandomSpawnPoint)))))

(event Game|Damage|EventAnyDamage
  (params (Damage :type Float%20%28single-precision%29) (DamageType :type Damage%20Type%20Object%20Reference) (InstigatedBy :type Controller%20Object%20Reference) (DamageCauser :type Actor%20Object%20Reference))
  (if (CallFunction|IsAlive)
    (bind _health (CallFunction|DecreaseHealth Damage))
    (if (== _health 0.0)
      (CallFunction|KillAI)
      (Utilities|FlowControl|Delay 5.0)
      (Actor|DestroyActor))))

(event EventTick
  (params (DeltaSeconds :type Float%20%28single-precision%29))
  (if (Math|Boolean|ANDBoolean (CallFunction|IsAlive) (CallFunction|IsPlayerAlive) (CallFunction|IsWithinAttackRange) (not (CallFunction|IsAttacking)))
    (CallFunction|DeactivateAIMovement)
    (if (CallFunction|IsPlayerAlive)
      (Animation|Montage|PlayMontage (Variables|Character|GetMesh) "/Game/Characters/Enemy_Spider/Animations/SpiderAttack01.SpiderAttack01" 0.5
        (:OnCompleted
          (CallFunction|ActivateAIMovement))))))

(fn ConstructionScript)

(fn IsWithinAttackRange
  (return (<= (Transformation|GetDistanceTo (Game|GetPlayerCharacter 0)) (Variables|Default|GetAttack%20Range))))

(fn IsAttacking
  (return (Animation|Montage|MontageIsPlaying (Components|SkeletalMesh|GetAnimInstance (Variables|Character|GetMesh)) "/Game/Characters/Enemy_Spider/Animations/SpiderAttack01.SpiderAttack01")))

(fn DeactivateAIMovement
  (bind _charactermovement (Variables|Character|GetCharacterMovement))
  (Components|Movement|StopMovementImmediately _charactermovement)
  (Components|Activation|Deactivate _charactermovement))

(fn ActivateAIMovement
  (Components|Activation|Activate (Variables|Character|GetCharacterMovement) false))

(fn DamagePlayer
  (if (CallFunction|IsAlive)
    (Game|Damage|ApplyDamage (Game|GetPlayerCharacter 0) (Variables|Default|GetDamage%20Per%20Hit) 0 0)))

(fn DecreaseHealth
  (params (Damage%20Taken :type Float%20%28single-precision%29))
  (bind _output_get (Variables|Default|SetHealth (Math|Float|Clamp(Float) (- (Variables|Default|GetHealth) Damage%20Taken) 0.0 (Variables|Default|GetMax%20Health))))
  (return _output_get))

(fn KillAI
  (bind _marine (CallFunction|Marine))
  (Variables|Default|SetIs%20Dead true)
  (CallFunction|DeactivateAIMovement)
  (Collision|SetActorEnableCollision false)
  (Default|IncreaseKills _marine)
  (Default|AddExperience _marine (Variables|Default|GetExperience%20Value))
  (CallFunction|RolltoSpawnPickup)
  (CallFunction|RemoveSpiderfromArray))

(fn Marine
  (bind _asbp_marine (Utilities|Casting|CastToBP_Marine (Game|GetPlayerCharacter 0)))
  (return _asbp_marine))

(fn IsAlive
  (return (not (Variables|Default|GetIs%20Dead))))

(fn RemoveSpiderfromArray
  (bind _asbp_game_mode (Utilities|Casting|CastToBP_GameMode (Game|GetGameMode))))

(fn RolltoSpawnPickup
  (if (<= (Math|Random|RandomIntegerinRange 0 100) (Variables|Default|GetPercent%20Chance%20To%20Spawn%20Pickup))
    (Game|SpawnActorfromClass "/Game/Blueprints/Pickups/BP_HealthPickup.BP_HealthPickup_C" (Transformation|GetActorTransform) "Undefined" 0 0)))

(fn IsPlayerAlive
  (return (Default|IsAlive (CallFunction|Marine))))