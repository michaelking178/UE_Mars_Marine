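; BP_Spider is an enemy spider character that chases the player and attacks up close.
; An AI MoveTo loop starts on BeginPlay and reissues one second after each success or failure.
; Tick checks distance against AttackRange, then pauses CharacterMovement while the attack montage plays, restoring it on completion.
; DamagePlayer applies DamagePerHit to the player but is not called within this Blueprint.
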(event EventBeginPlay
  (AI|AIMoveTo self "0, 0, 0" (Game|GetPlayerCharacter 0) 5.0 false :!label _label
    (:OnSuccess
      _)
    (:OnFail
      _))
  (Utilities|FlowControl|Delay 1.0)
  (goto _label))

(event EventTick
  (params (DeltaSeconds :type Float%20%28single-precision%29))
  (if (and (CallFunction|IsWithinAttackRange) (not (CallFunction|IsAttacking)))
    (CallFunction|DeactivateAIMovement)
    (Animation|Montage|PlayMontage (Variables|Character|GetMesh) "/Game/Characters/Enemy_Great_Spider/Animations/SpiderAttack01.SpiderAttack01"
      (:OnCompleted
        (CallFunction|ActivateAIMovement)))))

(fn ConstructionScript)

(fn IsWithinAttackRange
  (return (<= (Transformation|GetDistanceTo (Game|GetPlayerCharacter 0)) (Variables|Default|GetAttack%20Range))))

(fn IsAttacking
  (return (Animation|Montage|MontageIsPlaying (Components|SkeletalMesh|GetAnimInstance (Variables|Character|GetMesh)) "/Game/Characters/Enemy_Great_Spider/Animations/SpiderAttack01.SpiderAttack01")))

(fn DeactivateAIMovement
  (Components|Activation|Deactivate (Variables|Character|GetCharacterMovement)))

(fn ActivateAIMovement
  (Components|Activation|Activate (Variables|Character|GetCharacterMovement) false))

(fn DamagePlayer
  (Game|Damage|ApplyDamage (Game|GetPlayerCharacter 0) (Variables|Default|GetDamage%20Per%20Hit) 0 0))