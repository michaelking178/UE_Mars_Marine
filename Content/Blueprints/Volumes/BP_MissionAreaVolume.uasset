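; BP_MissionAreaVolume is a mission boundary volume that kills the player for staying outside it too long.
; Overlap begin and end events toggle IsOutsideMissionArea on the overlapping BP_Marine.
; Leaving starts a by-name timer of SecondsBeforePlayerDeath for Kill Player, and re-entering clears it.
; Kill Player applies MaxHealth as damage to player character 0, regardless of which marine triggered the timer.
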(event EventBeginPlay)

(event Collision|EventActorBeginOverlap
  (params (OtherActor :type Actor%20Object%20Reference))
  (bind _asbp_marine (Utilities|Casting|CastToBP_Marine OtherActor))
  (Variables|/Game/Blueprints/Pawns/BP_Marine.BP_Marine_C|SetIs%20Outside%20Mission%20Area _asbp_marine false)
  (Utilities|Time|ClearTimerbyFunctionName 0 "Kill Player"))

(event EventTick
  (params (DeltaSeconds :type Float%20%28single-precision%29)))

(event Collision|EventActorEndOverlap
  (params (OtherActor :type Actor%20Object%20Reference))
  (bind _asbp_marine (Utilities|Casting|CastToBP_Marine OtherActor))
  (Variables|/Game/Blueprints/Pawns/BP_Marine.BP_Marine_C|SetIs%20Outside%20Mission%20Area _asbp_marine true)
  (Utilities|Time|SetTimerbyFunctionName 0 "Kill Player" (Variables|Default|GetSeconds%20Before%20Player%20Death)))

(fn ConstructionScript)

(fn KillPlayer
  (bind _asbp_marine (Utilities|Casting|CastToBP_Marine (Game|GetPlayerCharacter 0)))
  (Game|Damage|ApplyDamage _asbp_marine (Variables|/Game/Blueprints/Pawns/BP_Marine.BP_Marine_C|GetMax%20Health _asbp_marine) 0 0))