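; Base weapon Blueprint that handles automatic firing and its audio for the owning Marine.
; StartFiring, if the Marine is alive, plays a fire sound, traces once, then loops the Marine's Weapon Trace on a timer at FireRate.
; StopFiring stops the stored sound, clears that timer and plays an end sound if the Marine is still alive.
; Hit tracing itself lives on the Marine, called by function name.
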(event EventBeginPlay)

(event Collision|EventActorBeginOverlap
  (params (OtherActor :type Actor%20Object%20Reference)))

(event EventTick
  (params (DeltaSeconds :type Float%20%28single-precision%29)))

(fn ConstructionScript)

(fn StartFiring
  (bind _marine (Variables|Default|GetMarine))
  (if (Default|IsAlive (Variables|Default|GetMarine))
    (bind _returnvalue (Audio|SpawnSound2D (Variables|Default|GetWeapon%20Fire%20Sound%20Cue) 1.0 1.0 0.0 0))
    (Variables|Default|SetWeapon%20Sound%20Component _returnvalue)
    (Default|WeaponTrace _marine)
    (Utilities|Time|SetTimerbyFunctionName _marine "Weapon Trace" (Variables|Default|GetFire%20Rate) true)))

(fn StopFiring
  (Utilities|IsValid (Variables|Default|GetWeapon%20Sound%20Component)
    (:Is%20Valid
      (Audio|Components|Audio|Stop (Variables|Default|GetWeapon%20Sound%20Component))
      (Utilities|Time|ClearTimerbyFunctionName (Variables|Default|GetMarine) "Weapon Trace")
      (if (Default|IsAlive (Variables|Default|GetMarine))
        (Audio|SpawnSound2D (Variables|Default|GetWeapon%20End%20Sound%20Cue) 1.0 1.0 0.0 0)))))